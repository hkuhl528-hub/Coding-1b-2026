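; BP_Door is a locked door that opens for the third-person player character when it holds at least one coin, which serves as a key.
; On actor overlap it casts to BP_ThirdPersonCharacter and checks TotalCoins.
; With a coin, it spends one and destroys its own mesh and box components, printing a success message.
; Without one, it prints a taunting message and stays in place.
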(event EventBeginPlay)

(event Collision|EventActorBeginOverlap
  (params (OtherActor :type Actor%20Object%20Reference))
  (bind _asbp_third_person_character (Utilities|Casting|CastToBP_ThirdPersonCharacter OtherActor))
  (if (> (Variables|/Game/ThirdPerson/Blueprints/BP_ThirdPersonCharacter.BP_ThirdPersonCharacter_C|GetTotalCoins _asbp_third_person_character) 0) ; If you have key, open door\nelse, laugh at them
    (Math|Integer|DecrementInt (Variables|/Game/ThirdPerson/Blueprints/BP_ThirdPersonCharacter.BP_ThirdPersonCharacter_C|GetTotalCoins _asbp_third_person_character)
      (:%20%20
        (Components|DestroyComponent (Variables|Default|GetSM_Bld_Door_01))
        (Components|DestroyComponent (Variables|Default|GetBox))
        (Development|PrintText "You found me!" true true "(R=0.222499,G=1.000000,B=0.252349,A=1.000000)")))
    (else
      (Development|PrintText "Get more keys lil bro"))))

(event EventTick
  (params (DeltaSeconds :type Float%20%28single-precision%29)))

(fn ConstructionScript)