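; BP_GrowingTree is a tree that grows in random steps after play begins.
; BeginPlay drives a looping DoN with a random limit, waiting a random few seconds before each Grow call.
; Grow adds a random amount to the tree mesh's relative scale.
; After each step, a DoN counter check either enables query and physics collision at zero or loops back for more growth.
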(event Custom|Grow
  (bind _sm_generic_tree_01 (Variables|Default|GetSM_Generic_Tree_01))
  (Transformation|SetRelativeScale3D _sm_generic_tree_01 (+ (Variables|/Script/Engine.SceneComponent|GetRelativeScale3D _sm_generic_tree_01) (Math|Random|RandomFloatinRange 0.1 0.5))))

(event EventBeginPlay
  (bind _counter (Utilities|FlowControl|DoN (Math|Random|RandomIntegerinRange 1 7) :!label _label)
    (:Exit
      (Utilities|FlowControl|Delay (Math|Random|RandomFloatinRange 2.5 5.0))
      (CallFunction|Grow)
      (if (== _counter 0)
        (Collision|SetCollisionEnabled (Variables|Default|GetSM_Generic_Tree_01) "QueryAndPhysics")
        (else
          (goto _label))))))

(fn ConstructionScript)